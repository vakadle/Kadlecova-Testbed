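; BP_NPC is an NPC Blueprint that shows dialog lines through a Talk event.
; Each call increments StartIndex and, while it is a valid index, reads that line from the StarDialog array.
; The line is printed for debugging and written to a WB_Dialog widget, which is created on first use and reused afterward.
; Nothing here resets the index or removes the widget when the lines run out.
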(event EventBeginPlay)

(event Collision|EventActorBeginOverlap
  (params (OtherActor :type Actor%20Object%20Reference)))

(event EventTick
  (params (DeltaSeconds :type Float%20%28single-precision%29)))

(event EventTalk
  (bind _startindex (Variables|Default|GetstartIndex))
  (bind _stardialog (Variables|Default|GetstarDialog))
  (bind _startindex_2 (Variables|Default|GetstartIndex))
  (bind _output (Utilities|Array|Get(acopy) _stardialog _startindex_2))
  (Math|Integer|IncrementInt _startindex
    (:%20%20
      (if (Utilities|Array|IsValidIndex _stardialog _startindex)
        (Development|PrintString _output)
        (Variables|Default|GetUI
          (:then
            _)
          (:else
            (bind _returnvalue (Game|ConstructObjectfromClass (Game|GetPlayerController 0) "/Game/NPC/WB_Dialog.WB_Dialog_C"))
            (bind _output_get (Variables|Default|SetUI _returnvalue))
            (UserInterface|Viewport|AddtoViewport _output_get 0)))
        (Variables|/Script/UMG.TextBlock|SetText (Variables|/Game/NPC/WB_Dialog.WB_Dialog_C|GetTalkText (Variables|Default|GetUI)) (Utilities|Text|ToText(String) _output))))))

(fn ConstructionScript)