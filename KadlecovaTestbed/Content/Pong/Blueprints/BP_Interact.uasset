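; BP_Interact is an interactable actor that shows a prompt widget while another actor overlaps it.
; The widget starts hidden on BeginPlay, appears on any actor's begin overlap and hides again on end overlap.
; Each tick it rotates the widget to face the player camera.
; The E key only prints a "Hello" debug string, with no overlap check in the graph.
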(event EventBeginPlay
  (Development|SetHiddeninGame (Variables|Default|GetWidget) true false))

(event Collision|EventActorBeginOverlap
  (params (OtherActor :type Actor%20Object%20Reference))
  (Development|SetHiddeninGame (Variables|Default|GetWidget) false false))

(event EventTick
  (params (DeltaSeconds :type Float%20%28single-precision%29))
  (bind _widget (Variables|Default|GetWidget))
  (Transformation|SetWorldRotation _widget (Math|Rotator|FindLookatRotation (Transformation|GetWorldLocation _widget) (Transformation|GetWorldLocation (Variables|/Script/Engine.Actor|GetRootComponent (Game|GetPlayerCameraManager 0)))) false false))

(event Collision|EventActorEndOverlap
  (params (OtherActor :type Actor%20Object%20Reference))
  (Development|SetHiddeninGame (Variables|Default|GetWidget) true false))

(event Input|KeyboardEvents|E
  (params (Key :type Key%20Structure :default "None"))
  (:Pressed
    (Development|PrintString "Hello")))

(fn ConstructionScript)